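; Player-controlled Blueprint that handles movement, camera look and casting of a glyph-built spell.
; BeginPlay adds the Enhanced Input mapping context and fills the Spell array with a hardcoded sequence of four glyphs.
; Shooting is gated by a Tick-driven timer against a fixed cooldown set on input, independent of glyph cooldowns.
; CastSpell spawns BP_SpellWeaver at the MagicSpawn transform and passes it the Spell array.
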(event `self.ReceiveBeginPlay`
  (bind _spell (`self.Spell`))
  ;[1 1 1] Controles
  (bind _asplayer_controller (cast `PlayerController` (`self.GetController`)))
  (bind _returnvalue (pcsubsystem `EnhancedInputLocalPlayerSubsystem` _asplayer_controller))
  (`/Engine/EditorBlueprintResources/StandardMacros.IsValid` _returnvalue
    (:`Is Valid`
      (`EnhancedInputSubsystemInterface.AddMappingContext` _returnvalue "/Game/Player/Inputs/IMC_Player.IMC_Player" 0 (struct))
      (`KismetArrayLibrary.Array_Add` _spell (make `/Game/Blueprints/MagicSystem_Data/Glyph` "NewEnumerator0" "NewEnumerator4" "NewEnumerator10" "NewEnumerator0" "NewEnumerator0" 0.0 300.0 0.0 30.0 1000.0 5.0))
      (`KismetArrayLibrary.Array_Add` _spell (make `/Game/Blueprints/MagicSystem_Data/Glyph` "NewEnumerator0" "NewEnumerator1" "NewEnumerator0" "NewEnumerator0" "NewEnumerator5" 0.0 0.0 0.0 0.0 1000.0))
      (`KismetArrayLibrary.Array_Add` _spell (make `/Game/Blueprints/MagicSystem_Data/Glyph` "NewEnumerator0" "NewEnumerator2" "NewEnumerator10" "NewEnumerator1" "NewEnumerator5" 5.0))
      (`KismetArrayLibrary.Array_Add` _spell (make `/Game/Blueprints/MagicSystem_Data/Glyph` "NewEnumerator0" "NewEnumerator1" "NewEnumerator3" "NewEnumerator0" "NewEnumerator5")))))

(event `EnhancedInput|/Game/Player/Inputs/IA_Look`
  (params (ActionValue :type "Vector2D Structure") (ElapsedSeconds :type "Float (double-precision)") (TriggeredSeconds :type "Float (double-precision)") (InputAction :type "InputAction Object Reference" :default "/Game/Player/Inputs/IA_Look.IA_Look"))
  ;[1 1 1] Controles
  (:`Triggered`
    (`self.AddControllerYawInput` ActionValue_X)
    (`self.AddControllerPitchInput` (* ActionValue_Y -1.0))))

(event `EnhancedInput|/Game/Player/Inputs/IA_Movement`
  (params (ActionValue :type "Vector2D Structure") (ElapsedSeconds :type "Float (double-precision)") (TriggeredSeconds :type "Float (double-precision)") (InputAction :type "InputAction Object Reference" :default "/Game/Player/Inputs/IA_Movement.IA_Movement"))
  (bind (_returnvalue_roll _returnvalue_pitch _returnvalue_yaw) (`KismetMathLibrary.BreakRotator` (`self.GetControlRotation`)))
  (bind (_returnvalue_roll_2 _returnvalue_pitch_2 _returnvalue_yaw_2) (`KismetMathLibrary.BreakRotator` (`self.GetControlRotation`)))
  ;[1 1 1] Controles
  (:`Triggered`
    (`self.AddMovementInput` (`KismetMathLibrary.GetRightVector` (`KismetMathLibrary.MakeRotator` _returnvalue_roll 0.0 _returnvalue_yaw)) ActionValue_X)
    (`self.AddMovementInput` (`KismetMathLibrary.GetForwardVector` (`KismetMathLibrary.MakeRotator` 0.0 0.0 _returnvalue_yaw_2)) ActionValue_Y)))

(event `EnhancedInput|/Game/Player/Inputs/IA_Shoot`
  (params (ActionValue :type Boolean) (ElapsedSeconds :type "Float (double-precision)") (TriggeredSeconds :type "Float (double-precision)") (InputAction :type "InputAction Object Reference" :default "/Game/Player/Inputs/IA_Shoot.IA_Shoot"))
  (:`Triggered`
    (set `self.Cooldown` 3.0)
    (if (>= (`self.CooldownTimer`) (`self.Cooldown`))
      (set `self.CooldownTimer` 0.0)
      (`self.CastSpell`))))

(event `self.ReceiveTick`
  (params (DeltaSeconds :type "Float (single-precision)"))
  (set `self.DeltaTime` DeltaSeconds)
  ;[1 1 1] Timer
  (set `self.CooldownTimer` (`KismetMathLibrary.FClamp` (+ (`self.DeltaTime`) (`self.CooldownTimer`)) 0.0 (`self.Cooldown`))))

(fn `CastSpell`
  (`|SpawnActorFromClass` "/Game/Blueprints/BP_SpellWeaver.BP_SpellWeaver_C" (`SceneComponent.K2_GetComponentToWorld` (`self.MagicSpawn`)) "AlwaysSpawn" "MultiplyWithRoot" null (`self.Spell`) null))

(fn `UserConstructionScript`)
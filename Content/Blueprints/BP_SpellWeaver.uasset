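; BP_SpellWeaver is a spell projectile actor that executes a queue of glyphs held in its InputSpell array.
; Each tick it interprets the first glyph (shoot, divide, timer or collision wait, element effect), removing it once done.
; Divide spawns copies of itself in a yaw fan, passing each the remaining glyphs and stats, then destroys the original, so spells branch recursively.
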(event `self.ReceiveBeginPlay`
  ;[1 1 1] Set OnHit Event to Set a boolean
  (set `self.WasHit` false)
  (add `self.OnActorHit` (delegate `OnActorHit_Event`)))

(event `OnActorHit_Event` :!signature `self.OnActorHit`
  (params (SelfActor :type "Actor Object Reference") (OtherActor :type "Actor Object Reference") (NormalImpulse :type "Vector Structure") (Hit :type "HitResult Structure (by ref)"))
  ;[1 1 1] Set OnHit Event to Set a boolean
  (set `self.WasHit` true))

(event `self.ReceiveTick`
  (params (DeltaSeconds :type "Float (single-precision)"))
  (set `self.DeltaTime` DeltaSeconds)
  (`self.Spell_Logic`))

(event `self.ProjectileMovement.OnProjectileStop`
  (params (ImpactResult :type "HitResult Structure (by ref)")))

(fn `CastSubSpell`
  (params (SubSpell_Transform :type "Transform Structure"))
  (locals (SubSpell :type "Array of /Game/Blueprints/MagicSystem_Data/Glyph Structure"))
  (bind _output_get (set `local.SubSpell` (`self.Input_Spell`)))
  (`KismetArrayLibrary.Array_Remove` _output_get)
  (bind _returnvalue (`|SpawnActorFromClass` "BP_SpellWeaver_C" SubSpell_Transform "AlwaysSpawn" "MultiplyWithRoot" null (`local.SubSpell`) (`KismetMathLibrary.GetForwardVector` (.rotation SubSpell_Transform)) (`self.Stats`) null))
  (`NiagaraComponent.SetAsset` (`/Game/Blueprints/BP_SpellWeaver.Niagara` _returnvalue) "/Game/Assets/FX/NS_Fire.NS_Fire" true))

(fn `Glyph_Division`
  (params (divisions :type "Float (double-precision)"))
  (bind _sphere (`self.Sphere`))
  (for _index (range (`KismetMathLibrary.FTrunc` divisions))
    (`self.CastSubSpell` (`KismetMathLibrary.MakeTransform` (`SceneComponent.K2_GetComponentLocation` _sphere) (`KismetMathLibrary.ComposeRotators` (`KismetMathLibrary.ComposeRotators` (`KismetMathLibrary.MakeRotFromX` (`SceneComponent.GetForwardVector` _sphere)) (`KismetMathLibrary.MakeRotator` 0.0 0.0 -45.0)) (`KismetMathLibrary.MakeRotator` 0.0 0.0 (* _index 45.0))))))
  (`self.K2_DestroyActor`))

(fn `Glyph_Shoot`
  (set `MovementComponent.Velocity` (* (`self.Direction`) (`.Speed_8_6015926348C025AD401C36B396959BFA` (break `/Game/Blueprints/MagicSystem_Data/Statistics` (`self.Stats`)))) (`self.ProjectileMovement`)))

(fn `Glyph_Timer`
  (params (Time :type "Float (double-precision)"))
  (if (`self.TempStarted`)
    (bind _output_get (set `self.Temp` (+ (`self.DeltaTime`) (`self.Temp`))))
    (if (>= _output_get Time)
      (set `self.TempStarted` false))
    (else
      (set `self.TempStarted` true)
      (set `self.Temp` 0.0))))

(fn `Spell_Logic`
  (bind _input_spell (`self.Input_Spell`))
  (bind (_type _action _triggers _element _wildcard) (break `/Game/Blueprints/MagicSystem_Data/Glyph` (`|GetArrayItem` _input_spell)))
  (if (`KismetArrayLibrary.Array_IsNotEmpty` _input_spell)
    ;[1 1 1] Igniter. Only one Igniter, Spell Start
    (switch `/Game/Blueprints/MagicSystem_Data/Glyph_Type` _type
      (:`NewEnumerator1`
        ;[1 1 1] Action
        (switch `/Game/Blueprints/MagicSystem_Data/Glyph_Actions` _action
          (:`NewEnumerator0`
            ;[1 1 1] Shoot
            (`self.Glyph_Shoot`)
            (`KismetArrayLibrary.Array_Remove` (`self.Input_Spell`) :!label _label))
          (:`NewEnumerator14`
            ;[1 1 1] Division Loop with primitive logic and primitib SubSpell Casting Function
            (`self.Glyph_Division` _wildcard))))
      (:`NewEnumerator2`
        ;[1 1 1] Triggers
        (switch `/Game/Blueprints/MagicSystem_Data/Glyph_Triggers` _triggers
          (:`NewEnumerator1`
            ;[1 1 1] Timer
            (if (`self.TempStarted`)
              (bind _output_get (set `self.Temp` (+ (`self.DeltaTime`) (`self.Temp`))))
              (if (>= _output_get _wildcard)
                (set `self.TempStarted` false)
                (goto _label))
              (else
                (set `self.TempStarted` true)
                (set `self.Temp` 0.0))))
          (:`NewEnumerator3`
            ;[1 1 1] Collision
            (if (`self.WasHit`)
              (set `self.WasHit` false)
              (goto _label)))))
      (:`NewEnumerator6`
        ;[1 1 1] Set Element
        (switch `/Game/Blueprints/MagicSystem_Data/Glyph_Elements` _element
          (:`NewEnumerator4`
            ;[1 1 1] Arcane - Default
            (`NiagaraComponent.SetAsset` (`self.Niagara`) "/Game/Assets/FX/NS_Fire.NS_Fire" true)
            (goto _label)))))))

(fn `UserConstructionScript`)